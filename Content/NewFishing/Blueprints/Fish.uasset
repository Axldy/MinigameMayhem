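; Fish actor for a fishing game that wanders inside the level's BoundingBox and can bite a FishLine.
; Every few seconds it picks a clamped random XY point at its current height, spawns a particle effect and glides there.
; Overlapping a FishLine stops movement and starts a WaitTime timer.
; If bait is still found when TakeBait fires, it notifies the line and sets itself as the fish on it.
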(event `self.ReceiveBeginPlay`
  (bind _returnvalue (`GameplayStatics.GetActorOfClass` "/Game/NewFishing/Blueprints/BoundingBox.BoundingBox_C"))
  (set `self.BoundingBox` _returnvalue)
  (`self.RandomMovement` :!label _label)
  (`KismetSystemLibrary.Delay` (`KismetMathLibrary.RandomFloatInRange` 4.0 6.0))
  (goto _label))

(event `RandomMovement`
  (if (not (`self.BaitFound`))
    (bind _point (`self.GetRandomPoint` :!label _label_2))
    (bind _output_get (set `self.TargetLocation` _point))
    (bind _boolean (`/Game/NewFishing/Blueprints/BoundingBox.IsPointInBoundingBox` (`self.BoundingBox`) _output_get))
    (if _boolean
      (`GameplayStatics.SpawnEmitterAtLocation` "/Game/StarterContent/Particles/P_Explosion.P_Explosion" (`self.K2_GetActorLocation`))
      (`KismetSystemLibrary.MoveComponentTo` (`self.DefaultSceneRoot`) (`self.TargetLocation`) (struct) false false (`KismetMathLibrary.RandomFloatInRange` 1.0 3.0) :!label _label_3)
      (else
        (goto _label_2)))))

(event `self.SphereCollision.OnComponentBeginOverlap`
  (params (OverlappedComponent :type "PrimitiveComponent Object Reference") (OtherActor :type "Actor Object Reference") (OtherComp :type "PrimitiveComponent Object Reference") (OtherBodyIndex :type Integer) (bFromSweep :type Boolean) (SweepResult :type "HitResult Structure (by ref)"))
  (if (== (`GameplayStatics.GetObjectClass` OtherActor) "/Game/NewFishing/Blueprints/Character/FishLine.FishLine_C")
    (bind _returnvalue (message `/Game/NewFishing/Blueprints/Interfaces/FishingInterface.GetFishLineObject` OtherActor))
    (set `self.Target` _returnvalue)
    (set `self.BaitFound` true)
    (`KismetSystemLibrary.K2_SetTimer` null "TakeBait" (`self.WaitTime`))
    (goto _label_3 :!via `Stop`)))

(event `self.SphereCollision.OnComponentEndOverlap`
  (params (OverlappedComponent :type "PrimitiveComponent Object Reference") (OtherActor :type "Actor Object Reference") (OtherComp :type "PrimitiveComponent Object Reference") (OtherBodyIndex :type Integer))
  (if (== OtherActor (`self.Target`))
    (set `self.BaitFound` false)
    (set `self.Target` null)))

(event `PrintValues`
  (`KismetSystemLibrary.PrintString` (`KismetStringLibrary.Concat_StrStr` "Weight: " (`KismetStringLibrary.Conv_DoubleToString` (`self.Weight`)) "kg")))

(fn `GetFishLineObject`
  (returns (ReturnValue :type "/Game/NewFishing/Blueprints/Character/FishLine Object Reference"))
  (return null))

(fn `GetRandomPoint`
  (returns (Point :type "Vector Structure"))
  (bind (_returnvalue_x _returnvalue_y _returnvalue_z) (`KismetMathLibrary.BreakVector` (`self.K2_GetActorLocation`)))
  (bind _boundingbox (`self.BoundingBox`))
  (bind (_returnvalue_x_2 _returnvalue_y_2) (`KismetMathLibrary.BreakVector` (`BoxComponent.GetScaledBoxExtent` (`/Game/NewFishing/Blueprints/BoundingBox.Box` _boundingbox))))
  (bind (_returnvalue_x_3 _returnvalue_y_3) (`KismetMathLibrary.BreakVector` (`SceneComponent.K2_GetComponentLocation` (`/Game/NewFishing/Blueprints/BoundingBox.DefaultSceneRoot` _boundingbox))))
  (return (`KismetMathLibrary.MakeVector` (`KismetMathLibrary.FClamp` (+ _returnvalue_x (`KismetMathLibrary.RandomFloatInRange` -200.0 200.0)) (- _returnvalue_x_3 _returnvalue_x_2) (+ _returnvalue_x_3 _returnvalue_x_2)) (`KismetMathLibrary.FClamp` (+ (`KismetMathLibrary.RandomFloatInRange` -200.0 200.0) _returnvalue_y) (- _returnvalue_y_3 _returnvalue_y_2) (+ _returnvalue_y_3 _returnvalue_y_2)) _returnvalue_z)))

(fn `TakeBait`
  (bind _target (`self.Target`))
  (if (`self.BaitFound`)
    (message `/Game/NewFishing/Blueprints/Interfaces/FishingInterface.BaitTaken` _target)
    (`/Game/NewFishing/Blueprints/Character/FishLine.SetFishOnLine` _target self)))

(fn `TakeFish`
  (returns (HasFish :type Boolean))
  (return false))

(fn `UserConstructionScript`)