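; FishLine is the cast fishing line actor, launched along its local X axis at a speed scaled by charge.
; On overlapping the WaterPlane, matched by display name, it destroys its projectile movement and snaps to the water's height.
; It holds the fish on the line and relays bait-taken events to the character.
; A hook attempt prints catch values or "Too Late!", then destroys fish and line and tells the GameMode to spawn fish.
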(event `self.ReceiveBeginPlay`)

(event `SetSpeed`
  (params (Charge :type "Float (double-precision)"))
  (bind _projectilemovement (`self.ProjectileMovement`))
  (`ProjectileMovementComponent.SetVelocityInLocalSpace` _projectilemovement (`KismetMathLibrary.MakeVector` (* Charge (`ProjectileMovementComponent.InitialSpeed` _projectilemovement)))))

(event `self.SphereCollision.OnComponentBeginOverlap`
  (params (OverlappedComponent :type "PrimitiveComponent Object Reference") (OtherActor :type "Actor Object Reference") (OtherComp :type "PrimitiveComponent Object Reference") (OtherBodyIndex :type Integer) (bFromSweep :type Boolean) (SweepResult :type "HitResult Structure (by ref)"))
  (bind (_returnvalue_x _returnvalue_y _returnvalue_z) (`KismetMathLibrary.BreakVector` (`self.K2_GetActorLocation` OtherActor)))
  (bind (_returnvalue_x_2 _returnvalue_y_2) (`KismetMathLibrary.BreakVector` (`self.K2_GetActorLocation`)))
  (if (`KismetStringLibrary.EqualEqual_StrStr` (`KismetSystemLibrary.GetDisplayName` OtherActor) "WaterPlane")
    (`ActorComponent.K2_DestroyComponent` (`self.ProjectileMovement`))
    (`self.K2_SetActorLocation` (`KismetMathLibrary.MakeVector` _returnvalue_x_2 _returnvalue_y_2 _returnvalue_z))))

(event `/Game/NewFishing/Blueprints/Interfaces/FishingInterface.BaitTaken`
  (message `/Game/NewFishing/Blueprints/Interfaces/FishingInterface.BaitTaken` (`self.Character`)))

(event `Hooked`
  (params (Success :type Boolean))
  (bind _returnvalue (`GameplayStatics.GetGameMode`))
  (bind _fish (`self.Fish`))
  (if Success
    (`/Game/NewFishing/Blueprints/Fish.PrintValues` _fish)
    (`self.K2_DestroyActor` _fish)
    (set `self.Fish` null)
    (`self.K2_DestroyActor`)
    (message `/Game/NewFishing/Blueprints/Interfaces/GameModeInterface.SpawnFish` _returnvalue)
    (else
      (`KismetSystemLibrary.PrintString` "Too Late!")
      (`self.K2_DestroyActor` _fish)
      (set `self.Fish` null)
      (`self.K2_DestroyActor`)
      (message `/Game/NewFishing/Blueprints/Interfaces/GameModeInterface.SpawnFish` _returnvalue))))

(fn `GetFishLineObject`
  (returns (ReturnValue :type "/Game/NewFishing/Blueprints/Character/FishLine Object Reference"))
  (return self))

(fn `SetFishOnLine`
  (params (Fish :type "/Game/NewFishing/Blueprints/Fish Object Reference"))
  (set `self.Fish` Fish))

(fn `TakeFish`
  (returns (HasFish :type Boolean))
  (return false))

(fn `UserConstructionScript`)