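; TimerComponent is a countdown timer that triggers game over when time runs out.
; On BeginPlay it resets CurrentTime to StartTime, then creates and displays a Timer widget.
; While unpaused, Tick accumulates delta time, decrements CurrentTime about once per second, updates the widget, and at zero pauses and calls CallGameOver.
; ResetTime restores only the count, without refreshing the widget or unpausing, and TogglePause flips the paused state.
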(event `self.ReceiveBeginPlay`
  (`self.ResetTime`)
  (bind _returnvalue (`|CreateWidget` "/Game/MigrateFolder/Blueprints/Character/Widgets/Timer.Timer_C"))
  (bind _output_get (set `self.TimerWidget` _returnvalue))
  (`/Game/MigrateFolder/Blueprints/Character/Widgets/Timer.UpdateTime` _output_get (`self.StartTime`))
  (`UserWidget.AddToViewport` _output_get 0))

(event `self.ReceiveTick`
  (params (DeltaSeconds :type "Float (single-precision)"))
  (if (not (`self.Paused`))
    (bind _output_get (set `self.SecondTimer` (+ DeltaSeconds (`self.SecondTimer`))))
    (if (>= _output_get 1.0)
      (set `self.SecondTimer` 0.0)
      (bind _result (`/Engine/EditorBlueprintResources/StandardMacros.DecrementInt` (`self.CurrentTime`))
        (:`  `
          (`/Game/MigrateFolder/Blueprints/Character/Widgets/Timer.UpdateTime` (`self.TimerWidget`) _result)
          (if (<= _result 0)
            (set `self.Paused` true)
            (`self.GameOver`)))))))

(event `ResetTime`
  (set `self.CurrentTime` (`self.StartTime`)))

(event `TogglePause`
  (set `self.Paused` (not (`self.Paused`))))