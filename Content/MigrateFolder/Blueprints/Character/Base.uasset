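; Base is a per-player fish drop-off actor that collects fish from its owning player.
; When an actor enters its Sphere, it checks that the instigator's player controller ID matches the base's PlayerIndex.
; On a match it calls TakeFishMessage on that actor, adds the returned count to FishAmount and prints the running total.
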(event `self.Sphere.OnComponentBeginOverlap`
  (params (OverlappedComponent :type "PrimitiveComponent Object Reference") (OtherActor :type "Actor Object Reference") (OtherComp :type "PrimitiveComponent Object Reference") (OtherBodyIndex :type Integer) (bFromSweep :type Boolean) (SweepResult :type "HitResult Structure (by ref)"))
  (bind _asplayer_controller (cast `PlayerController` (`self.GetInstigatorController` OtherActor)))
  (if (== (`GameplayStatics.GetPlayerControllerID` _asplayer_controller) (`self.PlayerIndex`))
    (bind _amount (message `/Game/MigrateFolder/Blueprints/Interfaces/FishingInterface.TakeFish` OtherActor))
    (bind _output_get (set `self.FishAmount` (+ _amount (`self.FishAmount`))))
    (`KismetSystemLibrary.PrintString` (`KismetStringLibrary.Conv_IntToString` _output_get))))

(fn `UserConstructionScript`)