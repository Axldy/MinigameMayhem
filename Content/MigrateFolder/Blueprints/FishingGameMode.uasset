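; Game mode for a fishing game that spawns fish, tracks points per player controller and ends the match on a timer.
; On BeginPlay it plays music, registers every controller in a points map and spawns the active fish count at random points within a BoundingBox actor at fixed height.
; AddPoints updates that map, while the timer component's GameOver event flags the finish and prints each Base's fish amount.
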(event `self.ReceiveBeginPlay`
  (bind _returnvalue (`GameplayStatics.GetActorOfClass` "/Game/MigrateFolder/Blueprints/BoundingBox.BoundingBox_C"))
  (set `self.Bounds` _returnvalue)
  (`GameplayStatics.PlaySound2D` "/Game/MigrateFolder/Blueprints/MusicCue.MusicCue" 1.0 1.0 0.0 null null)
  (`self.GetControllers`)
  (`self.SpawnAllFish`))

(event `self.SpawnFish`
  (bind _box (`/Game/MigrateFolder/Blueprints/BoundingBox.Box` (`self.Bounds`)))
  (bind (_returnvalue_x _returnvalue_y) (`KismetMathLibrary.BreakVector` (`SceneComponent.K2_GetComponentScale` _box)))
  (bind (_returnvalue_x_2 _returnvalue_y_2) (`KismetMathLibrary.BreakVector` (`KismetMathLibrary.RandomPointInBoundingBox` (0.0 0.0 125.0) (`BoxComponent.BoxExtent` _box))))
  (`|SpawnActorFromClass` "/Game/MigrateFolder/Blueprints/Fish.Fish_C" (`KismetMathLibrary.MakeTransform` (`KismetMathLibrary.MakeVector` (* _returnvalue_x_2 _returnvalue_x) (* _returnvalue_y_2 _returnvalue_y) 125.0)) "AlwaysSpawn" "OverrideRootScale" null null))

(event `SpawnAllFish`
  (for _ (range (`self.ActiveFish`))
    (`self.SpawnFish`)))

(event `SpawnPlayers`)

(event `self.AddPoints`
  (params (Controller :type "PlayerController Object Reference") (Points :type Integer))
  (bind (_value _returnvalue) (`BlueprintMapLibrary.Map_Find` (`self.PlayerPoints`) Controller))
  (if _returnvalue
    (`BlueprintMapLibrary.Map_Add` (`self.PlayerPoints`) Controller (+ Points _value))
    (`KismetSystemLibrary.PrintString` (`KismetStringLibrary.Concat_StrStr` (`KismetStringLibrary.Conv_IntToString` (`GameplayStatics.GetPlayerControllerID` Controller)) ":" (`KismetStringLibrary.Conv_IntToString` Points)))))

(event `self.TimerComponent.GameOver`
  (set `self.GameFinished` true)
  (`KismetSystemLibrary.PrintString` "Game Over")
  (bind _outactors (`GameplayStatics.GetAllActorsOfClass` "/Game/MigrateFolder/Blueprints/Character/Base.Base_C"))
  (for _array_element _outactors
    (`KismetSystemLibrary.PrintString` (`KismetStringLibrary.Conv_IntToString` (`/Game/MigrateFolder/Blueprints/Character/Base.FishAmount` _array_element)))))

(event `self.PauseTimer`
  (`/Game/MigrateFolder/Blueprints/TimerComponent.TogglePause` (`self.TimerComponent`)))

(fn `GetControllers`
  (bind _playerpoints (`self.PlayerPoints`))
  (bind _outactors (`GameplayStatics.GetAllActorsOfClass` "/Script/Engine.PlayerController"))
  (for _array_element _outactors
    (`BlueprintMapLibrary.Map_Add` _playerpoints _array_element))
  (bind _values (`BlueprintMapLibrary.Map_Values` _playerpoints))
  (for _array_element_2 _values
    (`KismetSystemLibrary.PrintString` (`KismetStringLibrary.Conv_IntToString` _array_element_2))))

(fn `UserConstructionScript`)