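; BoundingBox is an actor that defines a box volume for point containment tests and random point picking.
; IsPointInBoundingBox runs an axis-aligned test centred on the root's world location, using the Box extent multiplied by its world scale.
; RandomPointInBox samples each axis separately from the unscaled extent, then multiplies the resulting coordinate, origin included, by the world scale.
; The event graph and construction script are empty.
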(event `self.ReceiveActorBeginOverlap`
  (params (OtherActor :type "Actor Object Reference")))

(fn `IsPointInBoundingBox`
  (params (Point :type "Vector Structure"))
  (returns (Boolean :type Boolean))
  (bind _box (`self.Box`))
  (bind (_returnvalue_x _returnvalue_y _returnvalue_z) (`KismetMathLibrary.BreakVector` (`SceneComponent.K2_GetComponentScale` _box)))
  (bind (_boxextent_x _boxextent_y _boxextent_z) (`KismetMathLibrary.BreakVector` (`BoxComponent.BoxExtent` _box)))
  (return (`KismetMathLibrary.IsPointInBox` Point (`SceneComponent.K2_GetComponentLocation` (`self.DefaultSceneRoot`)) (`KismetMathLibrary.MakeVector` (* _returnvalue_x _boxextent_x) (* _returnvalue_y _boxextent_y) (* _returnvalue_z _boxextent_z)))))

(fn `RandomPointInBox`
  (returns (Location :type "Vector Structure"))
  (bind _box (`self.Box`))
  (bind (_returnvalue_x _returnvalue_y _returnvalue_z) (`KismetMathLibrary.BreakVector` (`SceneComponent.K2_GetComponentScale` _box)))
  (bind (_returnvalue_x_2 _returnvalue_y_2 _returnvalue_z_2) (`KismetMathLibrary.BreakVector` (`KismetMathLibrary.RandomPointInBoundingBox` (`SceneComponent.K2_GetComponentLocation` (`self.DefaultSceneRoot`)) (`BoxComponent.BoxExtent` _box))))
  (return (`KismetMathLibrary.MakeVector` (* _returnvalue_x_2 _returnvalue_x) (* _returnvalue_y_2 _returnvalue_y) (* _returnvalue_z_2 _returnvalue_z))))

(fn `UserConstructionScript`)