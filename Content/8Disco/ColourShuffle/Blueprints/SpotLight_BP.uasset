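; SpotLight_BP is a spotlight Blueprint for the ColourShuffle disco content, meant to show one of five named colours.
; A switch on ChosenColour records the colour in ColourOfLight and tints the SpotLight component blue, pink, orange, red or green.
; That switch is disconnected and never runs, so the SetLightColour event currently does nothing.
; The construction script is empty and Colours is unused.
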(event `SetLightColour`)

(fn `UserConstructionScript`)