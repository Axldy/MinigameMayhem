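; Platform actor for the ColourShuffle platform minigame that gives itself a random colour when play begins.
; A SetColour custom event picks one of five entries from the Colours array, stores it in ColourOfPlatform and applies the matching material to the Cube, with Pink using Magenta.
; The Cube is marked as a stand-in until a final mesh is available.
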(event `self.ReceiveBeginPlay`
  (`self.SetColour`))

(event `SetColour`
  ;[1 1 1] Set and Store Colour
  (switch `/Game/8Disco/ColourShuffle/Blueprints/PlatformMinigame/Colours` (`|GetArrayItem` (`self.Colours`) (`KismetMathLibrary.RandomIntegerInRange` 0 4))
    (:`NewEnumerator0`
      (set `self.ColourOfPlatform` "NewEnumerator0")
      ;;[1 1 1] Change when Mesh is available
      (`PrimitiveComponent.SetMaterial` (`self.Cube`) 0 (`self.Blue`)))
    (:`NewEnumerator1`
      (set `self.ColourOfPlatform` "NewEnumerator1")
      (`PrimitiveComponent.SetMaterial` (`self.Cube`) 0 (`self.Magenta`)))
    (:`NewEnumerator2`
      (set `self.ColourOfPlatform` "NewEnumerator2")
      (`PrimitiveComponent.SetMaterial` (`self.Cube`) 0 (`self.Orange`)))
    (:`NewEnumerator3`
      (set `self.ColourOfPlatform` "NewEnumerator3")
      (`PrimitiveComponent.SetMaterial` (`self.Cube`) 0 (`self.Red`)))
    (:`NewEnumerator4`
      (set `self.ColourOfPlatform` "NewEnumerator4")
      (`PrimitiveComponent.SetMaterial` (`self.Cube`) 0 (`self.Green`)))))

(fn `UserConstructionScript`)