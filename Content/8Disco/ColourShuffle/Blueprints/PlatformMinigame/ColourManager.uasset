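; Manager for the disco Colour Shuffle platform minigame, running its intro sequence, UI, music and endless rounds.
; Each round picks a random colour and runs a looping timer, then destroys non-matching platforms, removes the rest after a delay and respawns the grid.
; Each grid rebuild advances a round counter that enables random speakers to shoot from more sides or in fuller volleys, then holds at the hardest tier.
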(event `DisableInputToPlayers`
  ;[1 1 1] Couldn't get he players input to be disabled
  (bind _outactors (`GameplayStatics.GetAllActorsOfClass` "/Script/Engine.PlayerController"))
  (for _array_element _outactors
    (bind _outactors_2 (`GameplayStatics.GetAllActorsOfClass` "/Game/8Disco/ColourShuffle/Blueprints/ColourShuffleCharacter.ColourShuffleCharacter_C"))
    (for _array_element_2 _outactors_2
      (`self.DisableInput` _array_element_2 _array_element))))

(event `EnableInputToPlayers`
  (bind _outactors (`GameplayStatics.GetAllActorsOfClass` "/Script/Engine.PlayerController"))
  (for _array_element _outactors
    (bind _outactors_2 (`GameplayStatics.GetAllActorsOfClass` "/Game/8Disco/ColourShuffle/Blueprints/ColourShuffleCharacter.ColourShuffleCharacter_C"))
    (for _array_element_2 _outactors_2
      (`self.EnableInput` _array_element_2 _array_element)
      ;[1 1 1] Music Start
      (`/Engine/EditorBlueprintResources/StandardMacros.DoOnce` false
        (:`Completed`
          (bind _returnvalue (`GameplayStatics.CreateSound2D` "/Game/8Disco/ColourShuffle/Audio/DiscoLoopingTheme.DiscoLoopingTheme" 0.25 1.0 0.0 null))
          (`AudioComponent.Play` _returnvalue 0.0))))))

(event `self.ReceiveBeginPlay`
  (`self.Set-Up`)
  (`KismetSystemLibrary.Delay` 0.2)
  (`self.DisableInputToPlayers`))

(event `Set-Up`
  (`self.Create Grid`)
  (bind (_outactor _returnvalue) (`LevelSequencePlayer.CreateLevelSequencePlayer` "/Game/8Disco/ColourShuffle/IntroCutscene/Disco_MasterSequence.Disco_MasterSequence"))
  (`MovieSceneSequencePlayer.Play` _returnvalue)
  (add `MovieSceneSequencePlayer.OnFinished` _returnvalue (delegate `SequenceFinished`)))

(event `SequenceFinished`
  (bind _returnvalue (`|CreateWidget` "/Game/5VampireTag/ThirdPersonBP/Blueprints/StartGame_Widget.StartGame_Widget_C"))
  (`UserWidget.AddToViewport` _returnvalue 0)
  (`KismetSystemLibrary.Delay` 5.0)
  (bind _returnvalue_2 (`|CreateWidget` "/Game/8Disco/ColourShuffle/Blueprints/PlatformMinigame/UIColourMinigame.UIColourMinigame_C"))
  (bind _output_get (set `self.UI` _returnvalue_2))
  (`UserWidget.AddToViewport` _output_get 0)
  (`/Game/8Disco/ColourShuffle/Blueprints/PlatformMinigame/UIColourMinigame.Init` _output_get self)
  (`self.In-Game`))

(event `In-Game`
  (`self.EnableInputToPlayers`)
  (set `self.RoundOver?` false)
  (`self.SetChosenColour`)
  (`KismetSystemLibrary.K2_SetTimer` null "Timer" 1.0 true))

(event `SetChosenColour`
  ;[1 1 1] Set Chosen Colour
  (set `self.ChosenColour` (`|GetArrayItem` (`self.Colours`) (`KismetMathLibrary.RandomIntegerInRange` 0 4))))

(event `Timer`
  ;[1 1 1] Timer
  (set `self.TimePerRound` (- (`self.TimePerRound`) (`self.Second`)))
  (if (<= (`self.TimePerRound`) 0.0)
    (set `self.RoundOver?` true)
    (`KismetSystemLibrary.K2_ClearTimer` null "Timer")
    (`self.ResetRound`)))

(event `ResetRound`
  ;[1 1 1] Round Reset
  (set `self.TimePerRound` 5.0)
  (`self.Destroy Grid`))

(event `Change Colours`
  ;[1 1 1] Set Colours
  (bind _values (`BlueprintMapLibrary.Map_Values` (`self.GridMap`)))
  (for _array_element _values
    (`/Game/8Disco/ColourShuffle/Blueprints/PlatformMinigame/Platform.SetColour` _array_element)))

(event `Create Grid`
  ;[1 1 1] Grid Creation
  (set `self.RoundCounter` (+ (`self.RoundCounter`) 1))
  (`self.SetupSpeakers`)
  (for _index (range 1 (+ (`self.Rows`) 1))
    (for _index_2 (range 1 (+ (`self.Columns`) 1))
      (bind _returnvalue (`|SpawnActorFromClass` "/Game/8Disco/ColourShuffle/Blueprints/PlatformMinigame/Platform.Platform_C" (`KismetMathLibrary.MakeTransform` (`KismetMathLibrary.MakeVector` (* _index (`self.Offset X`)) (* _index_2 (`self.Offset Y`)))) "Undefined" "OverrideRootScale" null null))
      (`BlueprintMapLibrary.Map_Add` (`self.GridMap`) (make `/Game/8Disco/ColourShuffle/Blueprints/PlatformMinigame/Coordinates` _index _index_2) _returnvalue))))

(event `Destroy Grid`
  ;[1 1 1] Destroy Grid
  (`self.SetSpeakerSpawnerFalse`)
  (bind _values (`BlueprintMapLibrary.Map_Values` (`self.GridMap`)))
  (for _array_element _values
    (if (`|EnumInequality` (`/Game/8Disco/ColourShuffle/Blueprints/PlatformMinigame/Platform.ColourOfPlatform` _array_element) (`self.ChosenColour`))
      (`/Engine/EditorBlueprintResources/StandardMacros.IsValid` _array_element
        (:`Is Valid`
          (`self.K2_DestroyActor` _array_element)))
      (else
        (`KismetArrayLibrary.Array_Add` (`self.CorrectPlatforms`) _array_element))))
  (`KismetSystemLibrary.Delay` 1.0)
  (`self.DestroyRemaining`)
  (`self.Create Grid`)
  (`self.In-Game`))

(event `DestroyRemaining`
  ;[1 1 1] Destroy Grid
  (for _array_element (`self.CorrectPlatforms`)
    (`/Engine/EditorBlueprintResources/StandardMacros.IsValid` _array_element
      (:`Is Valid`
        (`self.K2_DestroyActor` _array_element)))))

(event `SetSpeakerSpawnerFalse`
  ;[1 1 1] Shooting Speakers
  (for _array_element (`self.Speakers`)
    (set `/Game/8Disco/ColourShuffle/Blueprints/Speaker_BP.IsEnabled?` false _array_element)))

(event `SetupSpeakers`
  ;[1 1 1] Shooting Speakers
  (switch `int` (`self.RoundCounter`)
    (:`1`
      (`self.SetSpeakerSpawnerFalse`))
    (:`2`
      (switch `int` (`KismetMathLibrary.RandomIntegerInRange` 0 1)
        (:`0`
          (`self.SpawnLeftSpeakers`))
        (:`1`
          (`self.SpawnRightSpeakers`))))
    (:`3`
      (switch `int` (`KismetMathLibrary.RandomIntegerInRange` 0 1)
        (:`0`
          (`self.SpawnTopSpeakers`))
        (:`1`
          (`self.SpawnBottomSpeakers`))))
    (:`4`
      (switch `int` (`KismetMathLibrary.RandomIntegerInRange` 0 1) :!label _label
        (:`0`
          (`self.SpawnLeftSpeakers`))
        (:`1`
          (`self.SpawnRightSpeakers`)))
      (switch `int` (`KismetMathLibrary.RandomIntegerInRange` 0 1)
        (:`0`
          (`self.SpawnTopSpeakers`))
        (:`1`
          (`self.SpawnBottomSpeakers`))))
    (:`5`
      (goto _label))
    (:`6`
      (switch `int` (`KismetMathLibrary.RandomIntegerInRange` 0 1)
        (:`0`
          (`self.SpawnLeftSpeakersFaster`))
        (:`1`
          (`self.SpawnRightSpeakersFaster`))))
    (:`7`
      (switch `int` (`KismetMathLibrary.RandomIntegerInRange` 0 1)
        (:`0`
          (`self.SpawnTopSpeakersFaster`))
        (:`1`
          (`self.SpawnBottomSpeakersFaster`))))
    (:`8`
      (switch `int` (`KismetMathLibrary.RandomIntegerInRange` 0 1) :!label _label_2
        (:`0`
          (`self.SpawnLeftSpeakersFaster`))
        (:`1`
          (`self.SpawnRightSpeakersFaster`)))
      (switch `int` (`KismetMathLibrary.RandomIntegerInRange` 0 1)
        (:`0`
          (`self.SpawnTopSpeakersFaster`))
        (:`1`
          (`self.SpawnBottomSpeakersFaster`)))
      (set `self.RoundCounter` 8))
    (:`9`
      (goto _label_2))))

(event `SpawnLeftSpeakers`
  (bind _leftspeakers (`self.LeftSpeakers`))
  ;[1 1 1] Shooting Speakers
  (`KismetArrayLibrary.Array_Shuffle` _leftspeakers)
  (for _index (range (+ (`KismetMathLibrary.RandomIntegerInRange` 1 2) 1))
    (bind _output (`|GetArrayItem` _leftspeakers _index))
    (set `/Game/8Disco/ColourShuffle/Blueprints/Speaker_BP.IsEnabled?` true _output)
    (`/Game/8Disco/ColourShuffle/Blueprints/Speaker_BP.Shoot` _output)))

(event `SpawnLeftSpeakersFaster`
  (bind _leftspeakers (`self.LeftSpeakers`))
  (`KismetArrayLibrary.Array_Shuffle` _leftspeakers)
  (for _index (range 3)
    (bind _output (`|GetArrayItem` _leftspeakers _index))
    (set `/Game/8Disco/ColourShuffle/Blueprints/Speaker_BP.IsEnabled?` true _output)
    (`/Game/8Disco/ColourShuffle/Blueprints/Speaker_BP.Shoot` _output)))

(event `SpawnTopSpeakers`
  (bind _topspeakers (`self.TopSpeakers`))
  ;[1 1 1] Shooting Speakers
  (`KismetArrayLibrary.Array_Shuffle` _topspeakers)
  (for _index (range (+ (`KismetMathLibrary.RandomIntegerInRange` 1 2) 1))
    (bind _output (`|GetArrayItem` _topspeakers _index))
    (set `/Game/8Disco/ColourShuffle/Blueprints/Speaker_BP.IsEnabled?` true _output)
    (`/Game/8Disco/ColourShuffle/Blueprints/Speaker_BP.Shoot` _output)))

(event `SpawnTopSpeakersFaster`
  (bind _topspeakers (`self.TopSpeakers`))
  (`KismetArrayLibrary.Array_Shuffle` _topspeakers)
  (for _index (range 3)
    (bind _output (`|GetArrayItem` _topspeakers _index))
    (set `/Game/8Disco/ColourShuffle/Blueprints/Speaker_BP.IsEnabled?` true _output)
    (`/Game/8Disco/ColourShuffle/Blueprints/Speaker_BP.Shoot` _output)))

(event `SpawnRightSpeakers`
  (bind _rightspeakers (`self.RightSpeakers`))
  ;[1 1 1] Shooting Speakers
  (`KismetArrayLibrary.Array_Shuffle` _rightspeakers)
  (for _index (range (+ (`KismetMathLibrary.RandomIntegerInRange` 1 2) 1))
    (bind _output (`|GetArrayItem` _rightspeakers _index))
    (set `/Game/8Disco/ColourShuffle/Blueprints/Speaker_BP.IsEnabled?` true _output)
    (`/Game/8Disco/ColourShuffle/Blueprints/Speaker_BP.Shoot` _output)))

(event `SpawnRightSpeakersFaster`
  (bind _rightspeakers (`self.RightSpeakers`))
  (`KismetArrayLibrary.Array_Shuffle` _rightspeakers)
  (for _index (range 3)
    (bind _output (`|GetArrayItem` _rightspeakers _index))
    (set `/Game/8Disco/ColourShuffle/Blueprints/Speaker_BP.IsEnabled?` true _output)
    (`/Game/8Disco/ColourShuffle/Blueprints/Speaker_BP.Shoot` _output)))

(event `SpawnBottomSpeakers`
  (bind _bottomspeakers (`self.BottomSpeakers`))
  ;[1 1 1] Shooting Speakers
  (`KismetArrayLibrary.Array_Shuffle` _bottomspeakers)
  (for _index (range (+ (`KismetMathLibrary.RandomIntegerInRange` 1 2) 1))
    (bind _output (`|GetArrayItem` _bottomspeakers _index))
    (set `/Game/8Disco/ColourShuffle/Blueprints/Speaker_BP.IsEnabled?` true _output)
    (`/Game/8Disco/ColourShuffle/Blueprints/Speaker_BP.Shoot` _output)))

(event `SpawnBottomSpeakersFaster`
  (bind _bottomspeakers (`self.BottomSpeakers`))
  (`KismetArrayLibrary.Array_Shuffle` _bottomspeakers)
  (for _index (range 3)
    (bind _output (`|GetArrayItem` _bottomspeakers _index))
    (set `/Game/8Disco/ColourShuffle/Blueprints/Speaker_BP.IsEnabled?` true _output)
    (`/Game/8Disco/ColourShuffle/Blueprints/Speaker_BP.Shoot` _output)))

(fn `UserConstructionScript`)