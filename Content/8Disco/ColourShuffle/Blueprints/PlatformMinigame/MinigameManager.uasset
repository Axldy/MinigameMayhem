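; Manager for the colour platform minigame, running repeating timed rounds on a spawned grid of platforms.
; Setup creates the UI widget, hands it a self reference and builds the grid map, then each round picks a random target colour.
; When the looping countdown expires, platforms of other colours are destroyed.
; After a short delay, the matching platforms are also removed, a fresh grid spawns and the next round starts.
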(event `self.ReceiveBeginPlay`
  (`self.Set-Up`))

(event `Set-Up`
  (bind _returnvalue (`|CreateWidget` "/Game/8Disco/ColourShuffle/Blueprints/PlatformMinigame/UIColourMinigame.UIColourMinigame_C"))
  (bind _output_get (set `self.UI` _returnvalue))
  (`UserWidget.AddToViewport` _output_get 0)
  (`/Game/8Disco/ColourShuffle/Blueprints/PlatformMinigame/UIColourMinigame.Init` _output_get self)
  (`self.Create Grid`)
  (`self.In-Game`))

(event `SetChosenColour`
  ;[1 1 1] Set Chosen Colour
  (set `self.ChosenColour` (`|GetArrayItem` (`self.Colours`) (`KismetMathLibrary.RandomIntegerInRange` 0 4))))

(event `In-Game`
  (set `self.RoundOver?` false)
  (`self.SetChosenColour`)
  (`KismetSystemLibrary.K2_SetTimer` null "Timer" 1.0 true))

(event `Timer`
  ;[1 1 1] Timer
  (set `self.TimePerRound` (- (`self.TimePerRound`) (`self.Second`)))
  (if (<= (`self.TimePerRound`) 0.0)
    (set `self.RoundOver?` true)
    (`KismetSystemLibrary.K2_ClearTimer` null "Timer")
    (`self.ResetRound`)))

(event `ResetRound`
  ;[1 1 1] Round Reset
  (set `self.TimePerRound` 5.0)
  (`self.Destroy Grid`))

(event `Change Colours`
  ;[1 1 1] Set Colours
  (bind _values (`BlueprintMapLibrary.Map_Values` (`self.Grid`)))
  (for _array_element _values
    (`/Game/8Disco/ColourShuffle/Blueprints/PlatformMinigame/Platform.SetColour` _array_element)))

(event `Create Grid`
  ;[1 1 1] Grid Creation
  (for _index (range 1 (+ (`self.Rows`) 1))
    (for _index_2 (range 1 (+ (`self.Columns`) 1))
      (bind _returnvalue (`|SpawnActorFromClass` "/Game/8Disco/ColourShuffle/Blueprints/PlatformMinigame/Platform.Platform_C" (`KismetMathLibrary.MakeTransform` (`KismetMathLibrary.MakeVector` (* _index (`self.Offset X`)) (* _index_2 (`self.Offset Y`)))) "Undefined" "OverrideRootScale" null null))
      (`BlueprintMapLibrary.Map_Add` (`self.Grid`) (make `/Game/8Disco/ColourShuffle/Blueprints/PlatformMinigame/Coordinates` _index _index_2) _returnvalue))))

(event `Destroy Grid`
  ;[1 1 1] Destroy Grid
  (bind _values (`BlueprintMapLibrary.Map_Values` (`self.Grid`)))
  (for _array_element _values
    (if (`|EnumInequality` (`/Game/8Disco/ColourShuffle/Blueprints/PlatformMinigame/Platform.ColourOfPlatform` _array_element) (`self.ChosenColour`))
      (`/Engine/EditorBlueprintResources/StandardMacros.IsValid` _array_element
        (:`Is Valid`
          (`self.K2_DestroyActor` _array_element)))
      (else
        (`KismetArrayLibrary.Array_Add` (`self.CorrectPlatforms`) _array_element))))
  (`KismetSystemLibrary.Delay` 1.0)
  (`self.DestroyRemaining`)
  (`self.Create Grid`)
  (`self.In-Game`))

(event `DestroyRemaining`
  ;[1 1 1] Destroy Grid
  (for _array_element (`self.CorrectPlatforms`)
    (`/Engine/EditorBlueprintResources/StandardMacros.IsValid` _array_element
      (:`Is Valid`
        (`self.K2_DestroyActor` _array_element)))))

(fn `UserConstructionScript`)