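; Game mode for the Colour Shuffle minigame that sets up local multiplayer on a shared camera.
; On BeginPlay it gathers spawn points, recreates the local players, then spawns and possesses a character for each controller tracked through login and logout.
; It reads the round length from MinigameInstance, but the countdown Timer is never started because its SetTimerByEvent node is disconnected.
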(event `self.ReceiveBeginPlay`
  (bind _outactors (`GameplayStatics.GetAllActorsOfClass` "/Game/Camera/BP_Camera.BP_Camera_C"))
  (set `self.Camera` (`|GetArrayItem` _outactors))
  (`self.SetUp`))

(event `SetUp`
  (`self.FindPlayerStarts`)
  (`self.SetUpControllers` (`self.NumberOfPlayers`))
  (`self.SetUpCharacters`)
  (`self.InGame`))

(event `InGame`
  (set `self.Time` (`/Game/MinigameInstance.TimePerGame` (cast `/Game/MinigameInstance` (`GameplayStatics.GetGameInstance`) :!pure true))))

(event `Timer`
  (set `self.Time` (- (`self.Time`) (`self.Second`)))
  (if (<= (`self.Time`) 0.0)
    (`KismetSystemLibrary.K2_ClearTimer` null "Timer")))

(event `self.K2_PostLogin`
  (params (NewPlayer :type "PlayerController Object Reference"))
  ;[1 1 1] Log Controllers
  (`KismetArrayLibrary.Array_Add` (`self.PlayerControllers`) NewPlayer))

(event `self.K2_OnLogout`
  (params (ExitingController :type "Controller Object Reference"))
  ;[1 1 1] Log Controllers
  (`KismetArrayLibrary.Array_RemoveItem` (`self.PlayerControllers`) (cast `/Game/CustomPlayerController` ExitingController :!pure true)))

(event `In-Game`)

(fn `FindPlayerStarts`
  (bind _outactors (`GameplayStatics.GetAllActorsOfClass` "/Game/Spawns/Spawn.Spawn_C"))
  (for _array_element _outactors
    (`KismetArrayLibrary.Array_Add` (`self.PlayerSpawns`) _array_element)))

(fn `SetUpCharacters`
  (for (_array_element _array_index) (`self.PlayerControllers`)
    (bind _returnvalue (`|SpawnActorFromClass` "/Game/8Disco/ColourShuffle/Blueprints/ColourShuffleCharacter.ColourShuffleCharacter_C" (`self.GetTransform` (`|GetArrayItem` (`self.PlayerSpawns`) _array_index)) "AdjustIfPossibleButAlwaysSpawn" "OverrideRootScale" null null))
    (`KismetArrayLibrary.Array_Add` (`self.ActivePlayers`) _returnvalue)
    (`Controller.Possess` _array_element _returnvalue)
    (bind _outactors (`GameplayStatics.GetAllActorsOfClass` "/Script/Engine.PlayerController"))
    (`PlayerController.SetViewTargetWithBlend` _outactors (`self.Camera`) 0.0 "VTBlend_Linear" 0.0 false)))

(fn `SetUpControllers`
  (params (NumberOfPlayers :type Integer))
  (`GameplayStatics.RemovePlayer` (`GameplayStatics.GetPlayerController` 0))
  (for _ (range NumberOfPlayers)
    (bind _returnvalue (`GameplayStatics.CreatePlayer` -1))))

(fn `UserConstructionScript`)