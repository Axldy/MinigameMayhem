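; Example game mode for the obstacle course that creates local players and spawns a character for each.
; A menu set-up event gathers Spawn actors, removes player 0 without destroying its pawn, then creates the requested number of players.
; PostLogin and OnLogout maintain the controller list, which drives spawning an ObstacleCharacter at a random spawn, possessing it and initializing its controller.
; Random spawn picks can repeat, with collision handling adjusting placement where possible.
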(event `self.ReceiveBeginPlay`
  (add `self.MenuSetUp` (delegate `MenuSetUp_Event`)))

(event `MenuSetUp_Event`
  (`self.FindPlayerStarts`)
  (`self.SetUpControllers` (`self.NumberOfPlayerrs`))
  (`self.SetUpCharacters`))

(event `self.K2_PostLogin`
  (params (NewPlayer :type "PlayerController Object Reference"))
  ;[1 1 1] Spawn Controllers
  (bind _returnvalue (`KismetArrayLibrary.Array_Add` (`self.PlayerControllers`) NewPlayer))
  (`KismetSystemLibrary.PrintString` (`KismetStringLibrary.Conv_IntToString` _returnvalue)))

(event `self.K2_OnLogout`
  (params (ExitingController :type "Controller Object Reference"))
  ;[1 1 1] Spawn Controllers
  (`KismetArrayLibrary.Array_RemoveItem` (`self.PlayerControllers`) (cast `/Game/9AaronsWork/Obstacle_Course/ObstacleBP/Blueprints/CustomPlayerController` ExitingController :!pure true)))

(fn `FindPlayerStarts`
  (bind _outactors (`GameplayStatics.GetAllActorsOfClass` "/Game/Spawns/Spawn.Spawn_C"))
  (for _array_element _outactors
    (`KismetArrayLibrary.Array_Add` (`self.PlayerSpawns`) _array_element)))

(fn `SetUpCharacters`
  (bind _playerspawns (`self.PlayerSpawns`))
  (for _array_element (`self.PlayerControllers`)
    (bind _returnvalue (`|SpawnActorFromClass` "/Game/9AaronsWork/Obstacle_Course/ObstacleBP/Blueprints/ObstacleCharacter.ObstacleCharacter_C" (`self.GetTransform` (`|GetArrayItem` _playerspawns (`KismetMathLibrary.RandomIntegerInRange` 0 (`KismetArrayLibrary.Array_LastIndex` _playerspawns)))) "AdjustIfPossibleButAlwaysSpawn" "OverrideRootScale" null null))
    (`Controller.Possess` _array_element _returnvalue)
    (`/Game/9AaronsWork/Obstacle_Course/ObstacleBP/Blueprints/CustomPlayerController.Init` (cast `/Game/9AaronsWork/Obstacle_Course/ObstacleBP/Blueprints/CustomPlayerController` _array_element :!pure true))))

(fn `SetUpControllers`
  (params (`Number of Players` :type Integer))
  (`GameplayStatics.RemovePlayer` (`GameplayStatics.GetPlayerController` 0))
  (for _ (range `Number of Players`)
    (bind _returnvalue (`GameplayStatics.CreatePlayer` -1))
    (`KismetSystemLibrary.PrintString` (`KismetSystemLibrary.GetDisplayName` _returnvalue))))

(fn `UserConstructionScript`)