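; Ladder actor for the obstacle course that toggles an ObstacleCharacter's climbing state through two overlap volumes.
; Entering the Box sets the character's OnLadder flag.
; Entering PingForwards clears the flag and launches the character along the Arrow's forward direction, overriding its velocity.
; A DoOnce gates the launch and resets two seconds after an overlap with PingForwards ends; any overlapping actor consumes it, as it precedes the cast.
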(event `self.Box.OnComponentBeginOverlap`
  (params (OverlappedComponent :type "PrimitiveComponent Object Reference") (OtherActor :type "Actor Object Reference") (OtherComp :type "PrimitiveComponent Object Reference") (OtherBodyIndex :type Integer) (bFromSweep :type Boolean) (SweepResult :type "HitResult Structure (by ref)"))
  (bind _asthird_person_character (cast `/Game/Obstacle_Course/ObstacleCharacterBP/Blueprints/ObstacleCharacter` OtherActor))
  (set `/Game/Obstacle_Course/ObstacleCharacterBP/Blueprints/ObstacleCharacter.OnLadder` true _asthird_person_character))

(event `self.PingForwards.OnComponentBeginOverlap`
  (params (OverlappedComponent :type "PrimitiveComponent Object Reference") (OtherActor :type "Actor Object Reference") (OtherComp :type "PrimitiveComponent Object Reference") (OtherBodyIndex :type Integer) (bFromSweep :type Boolean) (SweepResult :type "HitResult Structure (by ref)"))
  (`/Engine/EditorBlueprintResources/StandardMacros.DoOnce` false :!label _label
    (:`Completed`
      (bind _asthird_person_character (cast `/Game/Obstacle_Course/ObstacleCharacterBP/Blueprints/ObstacleCharacter` OtherActor))
      (set `/Game/Obstacle_Course/ObstacleCharacterBP/Blueprints/ObstacleCharacter.OnLadder` false _asthird_person_character)
      (`Character.LaunchCharacter` _asthird_person_character (* (`KismetMathLibrary.Conv_RotatorToVector` (`SceneComponent.K2_GetComponentRotation` (`self.Arrow`))) 1000.0) true true))))

(event `self.PingForwards.OnComponentEndOverlap`
  (params (OverlappedComponent :type "PrimitiveComponent Object Reference") (OtherActor :type "Actor Object Reference") (OtherComp :type "PrimitiveComponent Object Reference") (OtherBodyIndex :type Integer))
  (`KismetSystemLibrary.Delay` 2.0)
  (goto _label :!via `Reset`))

(fn `UserConstructionScript`)