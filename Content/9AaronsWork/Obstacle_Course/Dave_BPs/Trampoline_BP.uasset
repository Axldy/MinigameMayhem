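; Trampoline obstacle for the obstacle course that bounces an ObstacleCharacter upward.
; Overlapping the Box launches the character with TrampolineForce, overriding its vertical velocity.
; The PingForwards overlap events are empty, and a forward push along the Arrow's direction using PushForwardForce is left disconnected, so it never runs.
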(event `self.Box.OnComponentBeginOverlap`
  (params (OverlappedComponent :type "PrimitiveComponent Object Reference") (OtherActor :type "Actor Object Reference") (OtherComp :type "PrimitiveComponent Object Reference") (OtherBodyIndex :type Integer) (bFromSweep :type Boolean) (SweepResult :type "HitResult Structure (by ref)"))
  (bind _asthird_person_character (cast `/Game/Obstacle_Course/ObstacleCharacterBP/Blueprints/ObstacleCharacter` OtherActor))
  (`Character.LaunchCharacter` _asthird_person_character (`KismetMathLibrary.MakeVector` 0.0 0.0 (`self.TrampolineForce`)) false true))

(event `self.PingForwards.OnComponentBeginOverlap`
  (params (OverlappedComponent :type "PrimitiveComponent Object Reference") (OtherActor :type "Actor Object Reference") (OtherComp :type "PrimitiveComponent Object Reference") (OtherBodyIndex :type Integer) (bFromSweep :type Boolean) (SweepResult :type "HitResult Structure (by ref)")))

(event `self.PingForwards.OnComponentEndOverlap`
  (params (OverlappedComponent :type "PrimitiveComponent Object Reference") (OtherActor :type "Actor Object Reference") (OtherComp :type "PrimitiveComponent Object Reference") (OtherBodyIndex :type Integer)))

(fn `UserConstructionScript`)