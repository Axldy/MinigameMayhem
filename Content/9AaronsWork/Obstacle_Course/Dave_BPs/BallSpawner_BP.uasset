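; BallSpawner_BP repeatedly spawns RollingBall_BP actors from its location, in what the folder path places as an obstacle course.
; On BeginPlay it starts a looping timer whose interval is randomized once between SpawnMin and SpawnMax, so the spacing stays fixed afterward.
; Each spawn picks a preset world-Y offset at random and slightly varies the spawner's scale for the ball.
; Collision handling nudges blocked spawns or skips them.
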(event `self.ReceiveBeginPlay`
  (`KismetSystemLibrary.K2_SetTimerDelegate` (delegate `SpawnBalls`) (`KismetMathLibrary.RandomFloatInRange` (`self.SpawnMin`) (`self.SpawnMax`)) true))

(event `SpawnBalls`
  (bind _array (`|MakeArray` -200.0 -100.0 -50.0 0.0 50.0 100.0 200.0 :!type "Float (single-precision)"))
  (`|SpawnActorFromClass` "/Game/Obstacle_Course/Dave_BPs/RollingBall_BP.RollingBall_BP_C" (`KismetMathLibrary.MakeTransform` (+ (`self.K2_GetActorLocation`) (`KismetMathLibrary.MakeVector` 0.0 (`|GetArrayItem` _array (`KismetMathLibrary.RandomIntegerInRange` 0 (- (`KismetArrayLibrary.Array_Length` _array) 1))))) (struct) (* (`self.GetActorScale3D`) (`KismetMathLibrary.RandomFloatInRange` 0.75 1.25))) "AdjustIfPossibleButDontSpawnIfColliding" "OverrideRootScale" null null))

(fn `UserConstructionScript`)