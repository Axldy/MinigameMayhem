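; Base character Blueprint that broadcasts when its player is about to die or has reached the end.
; JustBeforeDeath and ReachEndOrder each wait a brief delay, then find every actor implementing I_PlayerDestroyed.
; Each of those actors receives the matching destroyed or reached-end interface message, passing the character's controller cast to CustomPlayerController.
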(event `JustBeforeDeath`
  (`KismetSystemLibrary.Delay` 0.02)
  (bind _outactors (`GameplayStatics.GetAllActorsWithInterface` "/Game/3DaveWork/I_PlayerDestroyed.I_PlayerDestroyed_C"))
  (for _array_element _outactors
    (message `/Game/3DaveWork/I_PlayerDestroyed.PlayerDestroyed` _array_element (cast `/Game/CustomPlayerController` (`self.GetController`) :!pure true))))

(event `ReachEndOrder`
  (`KismetSystemLibrary.Delay` 0.02)
  (bind _outactors (`GameplayStatics.GetAllActorsWithInterface` "/Game/3DaveWork/I_PlayerDestroyed.I_PlayerDestroyed_C"))
  (for _array_element _outactors
    (message `/Game/3DaveWork/I_PlayerDestroyed.PlayerReachedEnd` _array_element (cast `/Game/CustomPlayerController` (`self.GetController`) :!pure true))))

(fn `UserConstructionScript`)