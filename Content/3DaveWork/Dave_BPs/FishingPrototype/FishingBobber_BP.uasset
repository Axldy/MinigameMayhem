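; FishingBobber_BP is a fishing prototype bobber that flags the player's FishingCharacter as fishing while it waits for a bite.
; After a random delay of a few seconds, it spawns a Fish_BP near itself, passing a character reference, and destroys itself.
; A looping timer re-runs DestroyBobber, cancelling fishing and removing the bobber if the referenced character moves.
; A timeline-driven sinking motion is present but unconnected.
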(event `self.ReceiveBeginPlay`
  (`self.DestroyBobber`)
  (bind _asfishing_character (cast `/Game/3DaveWork/Dave_BPs/FishingPrototype/FishingCharacter` (`GameplayStatics.GetPlayerCharacter` 0)))
  (bind _output_get (set `self.As Third Person Character` _asfishing_character))
  (set `/Game/3DaveWork/Dave_BPs/FishingPrototype/FishingCharacter.IsFishing?` true _output_get)
  (`KismetSystemLibrary.Delay` (`KismetMathLibrary.RandomFloatInRange` 2.0 10.0))
  (`|SpawnActorFromClass` "/Game/3DaveWork/Dave_BPs/FishingPrototype/Fish_BP.Fish_BP_C" (`KismetMathLibrary.MakeTransform` (- (`self.K2_GetActorLocation`) (0.0 0.0 -20.0))) "Undefined" "OverrideRootScale" null (`self.TPCRef`) null)
  (`self.K2_DestroyActor`))

(event `DestroyBobber`
  (bind _returnvalue (`KismetSystemLibrary.K2_SetTimerDelegate` (delegate `DestroyBobber`) 0.1 true))
  (if (> (`KismetMathLibrary.VSize` (`MovementComponent.Velocity` (`Character.CharacterMovement` (`self.TPCRef`)))) 0.0)
    (set `/Game/3DaveWork/Dave_BPs/FishingPrototype/FishingCharacter.IsFishing?` false (`self.As Third Person Character`))
    (`self.K2_DestroyActor`)
    (`KismetSystemLibrary.K2_ClearAndInvalidateTimerHandle` _returnvalue)))

(fn `UserConstructionScript`)