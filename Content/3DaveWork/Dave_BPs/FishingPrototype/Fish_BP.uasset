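; Short-lived fish actor for the fishing prototype, which the player can catch before it disappears.
; On BeginPlay it flags and registers itself on the third-person character, then destroys itself after a brief random delay.
; Catch runs a timeline that lerps it toward the character with sweep.
; Box overlap with that character sets held weight, triggers the catch message, ends fishing and destroys the fish.
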(event `self.ReceiveBeginPlay`
  (set `/Game/3DaveWork/Dave_BPs/FishingPrototype/FishingCharacter.IsFish?` true (`self.As Third Person Character`))
  (`/Engine/EditorBlueprintResources/StandardMacros.IsValid` null
    (:`Is Valid`
      (`/Game/3DaveWork/Dave_BPs/FishingPrototype/FishingCharacter.FishRef` (`self.As Third Person Character`) self)
      (`KismetSystemLibrary.Delay` (`KismetMathLibrary.RandomFloatInRange` 0.8 1.7))
      (`self.K2_DestroyActor`))))

(event `self.Box.OnComponentBeginOverlap`
  (params (OverlappedComponent :type "PrimitiveComponent Object Reference") (OtherActor :type "Actor Object Reference") (OtherComp :type "PrimitiveComponent Object Reference") (OtherBodyIndex :type Integer) (bFromSweep :type Boolean) (SweepResult :type "HitResult Structure (by ref)"))
  (bind _as_third_person_character (`self.As Third Person Character`))
  (bind _as_third_person_character_2 (`self.As Third Person Character`))
  (`/Engine/EditorBlueprintResources/StandardMacros.IsValid` _as_third_person_character
    (:`Is Valid`
      (if (== _as_third_person_character OtherActor)
        (set `/Game/3DaveWork/Dave_BPs/FishingPrototype/FishingCharacter.FishWeightHeld` (+ (`/Game/3DaveWork/Dave_BPs/FishingPrototype/FishingCharacter.FishWeightHeld` (`self.As Third Person Character`)) (`KismetMathLibrary.RandomFloatInRange` (`self.MinFishWeight`) (`self.MaxFishWeight`))) (`self.As Third Person Character`))
        (message `/Game/3DaveWork/Dave_BPs/FishingPrototype/I_Fishing.Catch` _as_third_person_character_2)
        (set `/Game/3DaveWork/Dave_BPs/FishingPrototype/FishingCharacter.IsFishing?` false _as_third_person_character_2)
        (`self.K2_DestroyActor`)))))

(event `self.Catch`
  (bind (_direction _fishpullalpha) (`Timeline|PullFishIn` :!via `PlayFromStart`)
    (:`Update`
      (`self.K2_SetActorLocation` (`KismetMathLibrary.VLerp` (`self.K2_GetActorLocation`) (`self.K2_GetActorLocation` (`self.As Third Person Character`)) _fishpullalpha) true))))

(fn `GetFishLineObject`)

(fn `UserConstructionScript`)