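; Treadmill actor that pushes a FishingCharacter along its facing when the character overlaps its box.
; BeginPlay sets the root to one of four random right-angle rotations.
; On overlap, the PushPlayer timeline restarts and moves the capsule, with sweep, toward a point PushStrength ahead of MoveDirectionArrow.
; Each update lerps from player pawn 0's current location rather than a stored start or the overlapping character's own.
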(event `self.Box.OnComponentBeginOverlap`
  (params (OverlappedComponent :type "PrimitiveComponent Object Reference") (OtherActor :type "Actor Object Reference") (OtherComp :type "PrimitiveComponent Object Reference") (OtherBodyIndex :type Integer) (bFromSweep :type Boolean) (SweepResult :type "HitResult Structure (by ref)"))
  (bind _movedirectionarrow (`self.MoveDirectionArrow`))
  (bind _asfishing_character (cast `/Game/3DaveWork/Dave_BPs/FishingPrototype/FishingCharacter` OtherActor))
  (bind (_direction _pushplayer) (`Timeline|PushPlayer` :!via `PlayFromStart`)
    (:`Update`
      (`SceneComponent.K2_SetWorldLocation` (`Character.CapsuleComponent` _asfishing_character) (`KismetMathLibrary.VLerp` (`SceneComponent.K2_GetComponentLocation` (`Actor.RootComponent` (`GameplayStatics.GetPlayerPawn` 0))) (+ (`SceneComponent.K2_GetComponentLocation` _movedirectionarrow) (* (`KismetMathLibrary.GetForwardVector` (`SceneComponent.K2_GetComponentRotation` _movedirectionarrow)) (`self.PushStrength`))) _pushplayer) true false))))

(event `self.ReceiveBeginPlay`
  (`|ExecutionSequence`
    (:`then_0`
      (switch `int` (`KismetMathLibrary.RandomIntegerInRange` 0 3)
        (:`0`
          (set `self.Rotation` (struct)))
        (:`1`
          (set `self.Rotation` (struct :`Yaw` 90.0)))
        (:`2`
          (set `self.Rotation` (struct :`Yaw` 180.0)))
        (:`3`
          (set `self.Rotation` (struct :`Yaw` 270.0)))))
    (:`then_1`
      (`SceneComponent.K2_SetWorldRotation` (`self.DefaultSceneRoot`) (`self.Rotation`) false false))))

(fn `UserConstructionScript`)