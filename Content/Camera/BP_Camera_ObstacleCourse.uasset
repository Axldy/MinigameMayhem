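; Auto-scrolling camera actor for an obstacle course that also eliminates characters touching its trigger box.
; After a short delay at BeginPlay, a fast looping timer, rather than Tick, steps the actor steadily along world +X.
; Any ObstacleCharacter that begins overlapping the Box component is destroyed, with its name printed to screen.
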(event `self.ReceiveBeginPlay`
  (`parent.ReceiveBeginPlay`)
  (`KismetSystemLibrary.Delay` 3.0)
  (`KismetSystemLibrary.K2_SetTimerDelegate` (delegate `SetLocation`) 0.01 true))

(event `SetLocation`
  (bind (_returnvalue_x _returnvalue_y _returnvalue_z) (`KismetMathLibrary.BreakVector` (`self.K2_GetActorLocation`)))
  (if true
    (`self.K2_SetActorLocation` (`KismetMathLibrary.MakeVector` (+ _returnvalue_x 4.0) _returnvalue_y _returnvalue_z))))

(event `self.Box.OnComponentBeginOverlap`
  (params (OverlappedComponent :type "PrimitiveComponent Object Reference") (OtherActor :type "Actor Object Reference") (OtherComp :type "PrimitiveComponent Object Reference") (OtherBodyIndex :type Integer) (bFromSweep :type Boolean) (SweepResult :type "HitResult Structure (by ref)"))
  (bind _asobstacle_character (cast `/Game/9AaronsWork/Obstacle_Course/ObstacleBP/Blueprints/ObstacleCharacter` OtherActor))
  (`self.K2_DestroyActor` _asobstacle_character)
  (`KismetSystemLibrary.PrintString` (`KismetSystemLibrary.GetDisplayName` _asobstacle_character)))

(fn `UserConstructionScript`
  (`parent.UserConstructionScript`))