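; BP_lime is a lime hazard in a falling fruits game that kills the player character on overlap.
; Its Sphere1 overlap casts to FallingFruitCharacter, calls JustBeforeDeath, then destroys the character after a brief delay.
; It then resets the view by pointing all PlayerController actors at the level's BP_Camera.
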(event `self.Sphere1.OnComponentBeginOverlap`
  (params (OverlappedComponent :type "PrimitiveComponent Object Reference") (OtherActor :type "Actor Object Reference") (OtherComp :type "PrimitiveComponent Object Reference") (OtherBodyIndex :type Integer) (bFromSweep :type Boolean) (SweepResult :type "HitResult Structure (by ref)"))
  (bind _asfalling_fruit_character (cast `/Game/4FallingFruits/FallingFruits/Blueprints/FallingFruitCharacter` OtherActor))
  (`/Game/3DaveWork/BP_BaseCharacter.JustBeforeDeath` _asfalling_fruit_character)
  (`KismetSystemLibrary.Delay` 0.05)
  (`self.K2_DestroyActor` _asfalling_fruit_character)
  ;[1 1 1] ResetCamera
  (bind _returnvalue (`GameplayStatics.GetActorOfClass` "/Game/Camera/BP_Camera.BP_Camera_C"))
  (bind _outactors (`GameplayStatics.GetAllActorsOfClass` "/Script/Engine.PlayerController"))
  (`PlayerController.SetViewTargetWithBlend` _outactors _returnvalue 0.0 "VTBlend_Linear" 0.0 false))

(fn `UserConstructionScript`
  (`parent.UserConstructionScript`))