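; BP_Ball is a physics hazard ball that destroys the FallingFruitCharacter on contact.
; On BeginPlay it applies an impulse to its static mesh at the actor location, equal to its current velocity scaled by a random factor between Min and Max.
; When its sphere overlaps the character, it destroys that character and switches the player controller view target to the BP_Camera actor in the level.
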(event `self.ReceiveBeginPlay`
  ;[1 1 1] Set the life span and then the impulse
  (`PrimitiveComponent.AddImpulseAtLocation` (`self.StaticMesh`) (* (`self.GetVelocity`) (`KismetMathLibrary.RandomFloatInRange` (`self.Min`) (`self.Max`))) (`self.K2_GetActorLocation`) "None"))

(event `self.Sphere.OnComponentBeginOverlap`
  (params (OverlappedComponent :type "PrimitiveComponent Object Reference") (OtherActor :type "Actor Object Reference") (OtherComp :type "PrimitiveComponent Object Reference") (OtherBodyIndex :type Integer) (bFromSweep :type Boolean) (SweepResult :type "HitResult Structure (by ref)"))
  ;[1 1 1] When collides with player destroy the player
  (bind _asfalling_fruit_character (cast `/Game/4FallingFruits/FallingFruits/Blueprints/FallingFruitCharacter` OtherActor))
  (`self.K2_DestroyActor` _asfalling_fruit_character)
  ;;[1 1 1] ResetCamera
  (bind _returnvalue (`GameplayStatics.GetActorOfClass` "/Game/Camera/BP_Camera.BP_Camera_C"))
  (bind _outactors (`GameplayStatics.GetAllActorsOfClass` "/Script/Engine.PlayerController"))
  (`PlayerController.SetViewTargetWithBlend` _outactors _returnvalue 0.0 "VTBlend_Linear" 0.0 false))

(fn `UserConstructionScript`)