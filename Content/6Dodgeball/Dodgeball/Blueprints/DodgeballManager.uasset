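; Dodgeball match manager that switches the first player's view to a game camera and spawns local players at BeginPlay.
; SpawnPlayers creates players in a loop, sending each all four team messages in sequence and resetting the Player variables to None.
; It then prints a label based on Player1.
; A countdown that prints the timer and pauses the game at zero is present but disconnected, so it never runs.
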(event `self.ReceiveBeginPlay`
  ;[1 1 1] Set Game Camera
  (`PlayerController.SetViewTargetWithBlend` (`GameplayStatics.GetPlayerController` 0) (`self.GameCamera`) 0.0 "VTBlend_Linear" 0.0 false)
  (`self.SpawnPlayers`))

(event `self.ReceiveTick`
  (params (DeltaSeconds :type "Float (single-precision)"))
  ;[1 1 1] Timer
)

(fn `SpawnPlayers`
  (for _ (range 3)
    (bind _returnvalue (`GameplayStatics.CreatePlayer` -1))
    (`|ExecutionSequence`
      (:`then_0`
        (message `/Game/6Dodgeball/Dodgeball/Blueprints/Int_Teams.Set Team` _returnvalue "NewEnumerator0")
        (set `self.Player1` null))
      (:`then_1`
        (message `/Game/6Dodgeball/Dodgeball/Blueprints/Int_Teams.Set Team` _returnvalue "NewEnumerator1")
        (set `self.Player2` null))
      (:`then_2`
        (message `/Game/6Dodgeball/Dodgeball/Blueprints/Int_Teams.Set Team` _returnvalue "NewEnumerator2")
        (set `self.Player3` null))
      (:`then_3`
        (message `/Game/6Dodgeball/Dodgeball/Blueprints/Int_Teams.Set Team` _returnvalue "NewEnumerator3")
        (set `self.Player4` null))))
  (switch `/Game/6Dodgeball/Dodgeball/Blueprints/Players_Enum` "NewEnumerator1"
    (:`NewEnumerator1`
      (`KismetSystemLibrary.PrintString` "Player 1" true true (struct :`G` 0.78626 :`B` 1.0 :`A` 1.0)))
    (:`NewEnumerator2`
      (`KismetSystemLibrary.PrintString` "Player 2" true true (struct :`R` 1.0 :`B` 0.040099 :`A` 1.0)))
    (:`NewEnumerator3`
      (`KismetSystemLibrary.PrintString` "Player 3" true true (struct :`R` 0.061551 :`G` 1.0 :`A` 1.0)))
    (:`NewEnumerator4`
      (`KismetSystemLibrary.PrintString` "Player 4" true true (struct :`R` 1.0 :`G` 0.778582 :`A` 1.0)))))

(fn `UserConstructionScript`)