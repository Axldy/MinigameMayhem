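; Dodgeball projectile actor that detects when the ball directly strikes a player character.
; Each sphere hit increments a collision counter, and only a first collision with a DodgeballCharacter prints a message and sets the Hit flag.
; A later collision clears that flag after a short delay.
; The overlap event is an empty leftover, and disconnected nodes for carrying, throwing and destroying the ball never run.
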(event `self.Collision.OnComponentBeginOverlap`
  (params (OverlappedComponent :type "PrimitiveComponent Object Reference") (OtherActor :type "Actor Object Reference") (OtherComp :type "PrimitiveComponent Object Reference") (OtherBodyIndex :type Integer) (bFromSweep :type Boolean) (SweepResult :type "HitResult Structure (by ref)"))
  ;[1 1 1] Old Code
)

(event `self.Sphere.OnComponentHit`
  (params (HitComponent :type "PrimitiveComponent Object Reference") (OtherActor :type "Actor Object Reference") (OtherComp :type "PrimitiveComponent Object Reference") (NormalImpulse :type "Vector Structure") (Hit :type "HitResult Structure (by ref)"))
  ;[1 1 1] Interaction with ball
  (if (`self.Hit`)
    (`KismetSystemLibrary.Delay` 0.5)
    (set `self.Hit` false))
  (`/Engine/EditorBlueprintResources/StandardMacros.IncrementInt` (`self.CollisionCounter`)
    (:`  `
      (cast `/Game/6Dodgeball/Dodgeball/Blueprints/DodgeballCharacter` OtherActor)
      (if (== (`self.CollisionCounter`) 1)
        (`KismetSystemLibrary.PrintString` "Player Hit" true true (struct :`R` 1.0 :`B` 0.756324 :`A` 1.0))
        ;[1 1 1] Short delay after collision with player
        (set `self.Hit` true)))))

(fn `UserConstructionScript`)