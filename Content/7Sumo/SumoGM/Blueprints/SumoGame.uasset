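; Game mode for the local multiplayer Sumo minigame, a last-player-standing match on a breaking iceberg.
; It extends a parent state flow: setup creates local players, spawns characters on a shared camera and locks input through the intro sequence and countdown.
; Play starts the iceberg breaking and music until one character remains.
; Post-game awards points, plays the outro, then loads the main menu or next queued minigame by play mode.
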(event `self.K2_PostLogin`
  (params (NewPlayer :type "PlayerController Object Reference"))
  ;[1 1 1] Log Controllers
  (bind _returnvalue (`KismetArrayLibrary.Array_Add` (`self.PlayerControllers`) NewPlayer))
  (`KismetSystemLibrary.PrintString` (`KismetStringLibrary.Conv_IntToString` _returnvalue)))

(event `DisableInputToPlayers`
  ;[1 1 1] Disable/Enable Player input during cutscene
  (bind _outactors (`GameplayStatics.GetAllActorsOfClass` "/Script/Engine.PlayerController"))
  (for _array_element _outactors
    (bind _outactors_2 (`GameplayStatics.GetAllActorsOfClass` "/Game/7Sumo/SumoGM/Blueprints/SumoCharacter.SumoCharacter_C"))
    (for _array_element_2 _outactors_2
      (`self.DisableInput` _array_element_2 _array_element))
    (`self.SetPlayerColour`)))

(event `EnableInputToPlayers`
  ;[1 1 1] Disable/Enable Player input during cutscene
  (bind _outactors (`GameplayStatics.GetAllActorsOfClass` "/Script/Engine.PlayerController"))
  (for _array_element _outactors
    (bind _outactors_2 (`GameplayStatics.GetAllActorsOfClass` "/Game/7Sumo/SumoGM/Blueprints/SumoCharacter.SumoCharacter_C"))
    (for _array_element_2 _outactors_2
      (`self.EnableInput` _array_element_2 _array_element))))

(event `self.K2_OnLogout`
  (params (ExitingController :type "Controller Object Reference"))
  ;[1 1 1] Log Controllers
  (`KismetArrayLibrary.Array_RemoveItem` (`self.PlayerControllers`) (cast `PlayerController` ExitingController :!pure true)))

(event `self.ReceiveBeginPlay`
  (bind _outactors (`GameplayStatics.GetAllActorsOfClass` "/Game/Camera/BP_Camera.BP_Camera_C"))
  (set `self.Camera` (`|GetArrayItem` _outactors))
  (`self.ChangeGameState` "NewEnumerator0"))

(event `self.Set up`
  (`parent.Set up`)
  (`self.FindPlayerStarts`)
  (`self.SetUpControllers` (`self.NumberOfPlayers`))
  (`self.SetUpCharacters`)
  (`self.DisableInputToPlayers`)
  (bind (_outactor _returnvalue) (`LevelSequencePlayer.CreateLevelSequencePlayer` "/Game/7Sumo/IntroCutscene/Sumo_MasterSequence_Intro.Sumo_MasterSequence_Intro"))
  (`KismetSystemLibrary.Delay` 0.3) ; WAIT FOR GAME TO PAUSE WHEN CONTROL \nSCREEN IS SHOWN OTHERWISE MUSIC \nSTARTS PLAYING BEFORE GAME PAUSED
  (`MovieSceneSequencePlayer.Play` _returnvalue)
  (`/Engine/EditorBlueprintResources/StandardMacros.DoOnce` false
    (:`Completed`
      (`GameplayStatics.PlaySound2D` "/Game/Audio/Game_Start_Que.Game_Start_Que" 1.0 1.0 0.0 null null)
      (add `MovieSceneSequencePlayer.OnFinished` _returnvalue (delegate `CutsceneFinished`)))))

(event `CutsceneFinished`
  (bind _returnvalue (`|CreateWidget` "/Game/5VampireTag/ThirdPersonBP/Blueprints/StartGame_Widget.StartGame_Widget_C"))
  (`UserWidget.AddToViewport` _returnvalue 0)
  (`/Engine/EditorBlueprintResources/StandardMacros.DoOnce` false
    (:`Completed`
      (`GameplayStatics.PlaySound2D` "/Game/Audio/Beeping_Edit_Que.Beeping_Edit_Que" 1.0 1.0 0.0 null null)
      (`KismetSystemLibrary.Delay` 5.0)
      (`self.ChangeGameState` "NewEnumerator2"))))

(event `self.InGame`
  (`parent.InGame`)
  (`self.EnableInputToPlayers`)
  (`/Game/ArtLevels/SumoSmash/SM/Iceberg.Break Iceberg` (`self.Iceberg Ref`))
  ;[1 1 1] Music Start
  (`/Engine/EditorBlueprintResources/StandardMacros.DoOnce` false
    (:`Completed`
      (bind _returnvalue (`GameplayStatics.CreateSound2D` "/Game/7Sumo/Audio/SumoThemeLoop.SumoThemeLoop" 0.5 1.0 0.0 null))
      (`AudioComponent.Play` _returnvalue 0.0))))

(event `/Game/3DaveWork/I_PlayerDestroyed.PlayerDestroyed`
  (params (Controller :type "/Game/CustomPlayerController Object Reference"))
  (bind _activeplayers (`self.ActivePlayers`))
  (`parent.PlayerDestroyed` Controller)
  (bind _assumo_character (cast `/Game/7Sumo/SumoGM/Blueprints/SumoCharacter` (`Controller.K2_GetPawn` Controller)))
  (`KismetArrayLibrary.Array_RemoveItem` _activeplayers _assumo_character)
  (if (== (`KismetArrayLibrary.Array_Length` _activeplayers) 1)
    (`self.ChangeGameState` "NewEnumerator3")))

(event `self.PostGame`
  (`parent.PostGame`)
  (bind _outactors (`GameplayStatics.GetAllActorsOfClass` "/Game/CustomPlayerController.CustomPlayerController_C"))
  (for _array_element _outactors
    (bind _outactors_2 (`GameplayStatics.GetAllActorsOfClass` "/Game/7Sumo/SumoGM/Blueprints/SumoCharacter.SumoCharacter_C"))
    (for _array_element_2 _outactors_2
      (`self.DisableInput` _array_element_2 _array_element))
    (`/Engine/EditorBlueprintResources/StandardMacros.DoOnce` false
      (:`Completed`
        (bind _ascustom_player_controller (cast `/Game/CustomPlayerController` _array_element :!pure true))
        (set `/Game/CustomPlayerController.PersonalScore` (+ (`/Game/CustomPlayerController.PersonalScore` _ascustom_player_controller) 3) _ascustom_player_controller)
        (bind _returnvalue (`|CreateWidget` "/Game/5VampireTag/ThirdPersonBP/Blueprints/EndGame_Widget.EndGame_Widget_C"))
        (`UserWidget.AddToViewport` _returnvalue 0)
        (bind (_outactor _returnvalue_2) (`LevelSequencePlayer.CreateLevelSequencePlayer` "/Game/5VampireTag/IntroCutscene/Tag_OutroCinematicCutscene_01.Tag_OutroCinematicCutscene_01"))
        (`MovieSceneSequencePlayer.Play` _returnvalue_2)
        (`KismetSystemLibrary.Delay` 5.0)
        (`GameplayStatics.SetGamePaused` true)
        (bind _asminigame_instance (cast `/Game/MinigameInstance` (`GameplayStatics.GetGameInstance`)))
        (switch `/Game/UI/PlayMode` (`/Game/MinigameInstance.PlayMode` _asminigame_instance)
          (:`NewEnumerator0`
            (`GameplayStatics.OpenLevelBySoftObjectPtr` "/Game/UI/MainMenu/MainMenu.MainMenu"))
          (:`NewEnumerator1`
            (`/Game/MinigameInstance.LoadNextInQueue` _asminigame_instance :!label _label))
          (:`NewEnumerator2`
            (goto _label)))))))

(event `Timer`
  ;[1 1 1] Redundant
  (set `self.Time` (- (`self.Time`) (`self.Second`)))
  (if (<= (`self.Time`) 0.0)
    (`KismetSystemLibrary.K2_ClearTimer` null "Timer")))

(fn `FindPlayerStarts`
  (bind _outactors (`GameplayStatics.GetAllActorsOfClass` "/Game/Spawns/Spawn.Spawn_C"))
  (for _array_element _outactors
    (`KismetArrayLibrary.Array_Add` (`self.PlayerSpawns`) _array_element)))

(fn `SetUpCharacters`
  (for (_array_element _array_index) (`self.PlayerControllers`)
    (bind _returnvalue (`|SpawnActorFromClass` "/Game/7Sumo/SumoGM/Blueprints/SumoCharacter.SumoCharacter_C" (`self.GetTransform` (`|GetArrayItem` (`self.PlayerSpawns`) _array_index)) "AdjustIfPossibleButAlwaysSpawn" "OverrideRootScale" null null))
    (`KismetArrayLibrary.Array_Add` (`self.ActivePlayers`) _returnvalue)
    (`Controller.Possess` _array_element _returnvalue)
    (bind _outactors (`GameplayStatics.GetAllActorsOfClass` "/Script/Engine.PlayerController"))
    (`PlayerController.SetViewTargetWithBlend` _outactors (`self.Camera`) 0.0 "VTBlend_Linear" 0.0 false)))

(fn `SetUpControllers`
  (params (NumberOfPlayers :type Integer))
  (`GameplayStatics.RemovePlayer` (`GameplayStatics.GetPlayerController` 0))
  (for _ (range NumberOfPlayers)
    (bind _returnvalue (`GameplayStatics.CreatePlayer` -1))
    (`KismetSystemLibrary.PrintString` (`KismetSystemLibrary.GetDisplayName` _returnvalue))))

(fn `UserConstructionScript`)